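; BP_CuboBarco is a player-controlled vehicle, named as a cube boat, driven with Enhanced Input.
; On BeginPlay it adds IMC_Default to the player's input subsystem, printing an error if the controller or subsystem check fails.
; W/S actions call Accelerate/Deccelerate and A/D call Turn with a direction flag; these functions are defined outside this graph.
; The look action yaws the SpringArm to orbit the camera around the vehicle.
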(event `self.ReceiveBeginPlay`
  (bind _asplayer_controller (cast `PlayerController` (`self.GetController`))
    (:`then`
      (bind _returnvalue (pcsubsystem `EnhancedInputLocalPlayerSubsystem` _asplayer_controller))
      (`/Engine/EditorBlueprintResources/StandardMacros.IsValid` _returnvalue
        (:`Is Valid`
          (`EnhancedInputSubsystemInterface.AddMappingContext` _returnvalue "/Game/ThirdPerson/Input/IMC_Default.IMC_Default" 0 (struct)))
        (:`Is Not Valid`
          (`KismetSystemLibrary.PrintString` "ERRORSITO" true true (struct :`R` 1.0 :`G` 0.040707 :`A` 1.0)))))
    (:`CastFailed`
      (`KismetSystemLibrary.PrintString` "ERRORSITO"))))

(event `EnhancedInput|/Game/ThirdPerson/Input/Actions/IA_W`
  (params (ActionValue :type Boolean) (ElapsedSeconds :type "Float (double-precision)") (TriggeredSeconds :type "Float (double-precision)") (InputAction :type "InputAction Object Reference" :default "/Game/ThirdPerson/Input/Actions/IA_W.IA_W"))
  (:`Triggered`
    (`self.Accelerate`)))

(event `EnhancedInput|/Game/ThirdPerson/Input/Actions/IA_D`
  (params (ActionValue :type Boolean) (ElapsedSeconds :type "Float (double-precision)") (TriggeredSeconds :type "Float (double-precision)") (InputAction :type "InputAction Object Reference" :default "/Game/ThirdPerson/Input/Actions/IA_D.IA_D"))
  (:`Triggered`
    (`self.Turn` true)))

(event `EnhancedInput|/Game/ThirdPerson/Input/Actions/IA_S`
  (params (ActionValue :type Boolean) (ElapsedSeconds :type "Float (double-precision)") (TriggeredSeconds :type "Float (double-precision)") (InputAction :type "InputAction Object Reference" :default "/Game/ThirdPerson/Input/Actions/IA_S.IA_S"))
  (:`Triggered`
    (`self.Deccelerate`)))

(event `EnhancedInput|/Game/ThirdPerson/Input/Actions/IA_A`
  (params (ActionValue :type Boolean) (ElapsedSeconds :type "Float (double-precision)") (TriggeredSeconds :type "Float (double-precision)") (InputAction :type "InputAction Object Reference" :default "/Game/ThirdPerson/Input/Actions/IA_A.IA_A"))
  (:`Triggered`
    (`self.Turn` false)))

(event `EnhancedInput|/Game/VehicleTemplate/Input/Actions/IA_LookAround`
  (params (ActionValue :type "Float (double-precision)") (ElapsedSeconds :type "Float (double-precision)") (TriggeredSeconds :type "Float (double-precision)") (InputAction :type "InputAction Object Reference" :default "/Game/VehicleTemplate/Input/Actions/IA_LookAround.IA_LookAround"))
  (:`Triggered`
    (`SceneComponent.K2_AddLocalRotation` (`self.SpringArm`) (`KismetMathLibrary.MakeRotator` 0.0 0.0 ActionValue) false false) ; Rotate camera around the vehicle
  ))

(fn `UserConstructionScript`)